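; BP_Skalierungsfaktoren is an interactive math visual that shows two scaled arrow vectors and their resultant, with German "Skalierung" (scaling) labels.
; Each Tick maps two slider values to the Y and Z arrow lengths and shows each length relative to its BeginPlay value.
; A third arrow takes the Pythagorean length and rotates toward the vector sum.
; The labels call ArrowY "X" and ArrowZ "Y".
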(event `self.ReceiveBeginPlay`
  (set `self.ArrowZStartLength` (`ArrowComponent.ArrowLength` (`self.ArrowZ`)))
  (set `self.ArrowY Start Length` (`ArrowComponent.ArrowLength` (`self.ArrowY`))))

(event `self.ReceiveTick`
  (params (DeltaSeconds :type "Float (single-precision)"))
  (bind _arrowpointlength (`self.ArrowPointLength`))
  (bind _arrowz (`self.ArrowZ`))
  (bind _arrowy (`self.ArrowY`))
  (`TextRenderComponent.K2_SetText` (`self.TextRender1`) (`|FormatText` "Skalierung Y: {Value}" (/ (`ArrowComponent.ArrowLength` (`self.ArrowZ`)) (`self.ArrowZStartLength`))))
  (`TextRenderComponent.K2_SetText` (`self.TextRender2`) (`|FormatText` "Skalierung X: {Value}" (/ (`ArrowComponent.ArrowLength` (`self.ArrowY`)) (`self.ArrowY Start Length`))))
  (set `ArrowComponent.ArrowLength` (`KismetMathLibrary.FClamp` (`KismetMathLibrary.MapRangeClamped` (`/Game/Global/Blueprints/BP_Slider.Value` (`self.SliderForY`)) 0.0 1.0 80.0 (`self.MaxArrowLenght`)) 80.0 (`self.MaxArrowLenght`)) (`self.ArrowY`))
  (set `ArrowComponent.ArrowLength` (`KismetMathLibrary.FClamp` (`KismetMathLibrary.MapRangeClamped` (`/Game/Global/Blueprints/BP_Slider.Value` (`self.SliderForZ`)) 0.0 1.0 80.0 (`self.MaxArrowLenght`)) 80.0 (`self.MaxArrowLenght`)) (`self.ArrowZ`))
  (set `ArrowComponent.ArrowLength` (`KismetMathLibrary.Sqrt` (+ (`KismetMathLibrary.MultiplyMultiply_FloatFloat` (`ArrowComponent.ArrowLength` (`self.ArrowY`)) 2.0) (`KismetMathLibrary.MultiplyMultiply_FloatFloat` (`ArrowComponent.ArrowLength` (`self.ArrowZ`)) 2.0))) (`self.ArrowPointLength`))
  (`SceneComponent.K2_SetWorldRotation` _arrowpointlength (`KismetMathLibrary.FindLookAtRotation` (`SceneComponent.K2_GetComponentLocation` _arrowpointlength) (+ (* (`KismetMathLibrary.Normal` (`SceneComponent.GetForwardVector` _arrowy)) (`ArrowComponent.ArrowLength` _arrowy)) (* (`KismetMathLibrary.Normal` (`SceneComponent.GetForwardVector` _arrowz)) (`ArrowComponent.ArrowLength` _arrowz)) (`self.K2_GetActorLocation`))) false false))

(fn `UserConstructionScript`)